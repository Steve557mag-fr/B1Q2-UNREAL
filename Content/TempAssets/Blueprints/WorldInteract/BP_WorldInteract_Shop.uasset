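; Interactable shop actor with a Wanderer merchant that greets the player and opens the shop.
; OnInteract aims the player's camera at the shop's Arrow, hides the player mesh and plays the enter montage.
; A DoOnce gates entry and the shop toggle on the GameMode, until PlayAnimationGoodbye plays the farewell, closes the shop and resets it.
; Purchase calls for souls and items are unconnected placeholder nodes.
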(event `PlayAnimationEnter`
  (`/Engine/EditorBlueprintResources/StandardMacros.DoOnce` false :!label _label
    (:`Completed`
      (`|PlayMontage` (`self.Wanderer`) "/Game/TempAssets/Animations/Wanderer/AM_Enter.AM_Enter"
        (:`then`
          (message `/Game/TempAssets/Blueprints/BPInterfaces/BPI_Interface.ToggleShop` (`GameplayStatics.GetGameMode`) true))))))

(event `PlayAnimationGoodbye`
  (`|PlayMontage` (`self.Wanderer`) "/Game/TempAssets/Animations/Wanderer/AM_Goodbye.AM_Goodbye"
    (:`then`
      (message `/Game/TempAssets/Blueprints/BPInterfaces/BPI_Interface.ToggleShop` (`GameplayStatics.GetGameMode`) false)
      (goto _label :!via `Reset`))))

(fn `OnInteract`
  (message `/Game/TempAssets/Blueprints/BPInterfaces/BPI_Character.LookAt` (`GameplayStatics.GetPlayerCharacter` 0) (`SceneComponent.K2_GetComponentToWorld` (`self.Arrow`)) false)
  (`self.PlayAnimationEnter`))

(fn `UserConstructionScript`
  (`parent.UserConstructionScript`))