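; Base Blueprint for world interactables that the player triggers by pressing interact while standing inside their overlap area.
; Actor overlap events use a BP_Player class check to set IsPlayerInside and show or hide the player's EmoteInteract prompt.
; BeginPlay binds TriggerEvent to player 0's InteractPressed event, so every instance hears the press but only those with the player inside call OnInteract.
; OnInteract is empty here, serving as the hook for child classes.
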(event `self.ReceiveActorBeginOverlap`
  (params (OtherActor :type "Actor Object Reference"))
  ;[1 1 1] Detection du joueur
  ;;[1 1 1] Verifier que ce soit le joueur
  (if (`self.IsPlayer` OtherActor)
    ;;[1 1 1] Si oui alors, assigner à vrai
    (set `self.isPlayerInside` true)
    ;;[1 1 1] Rendre visible le btn d'interaction
    (bind _asbp_player (cast `/Game/TempAssets/Blueprints/Player/BP_Player` OtherActor))
    (`SceneComponent.SetVisibility` (`/Game/TempAssets/Blueprints/Player/BP_Player.Emote Interact` _asbp_player) true false)))

(event `self.ReceiveActorEndOverlap`
  (params (OtherActor :type "Actor Object Reference"))
  ;[1 1 1] Detection du joueur
  ;;[1 1 1] Verifier que ce soit le joueur
  (if (`self.IsPlayer` OtherActor)
    ;;[1 1 1] Si oui alors, assigner à faux
    (set `self.isPlayerInside` false)
    ;;[1 1 1] Rendre invisible le btn d'interaction
    (bind _asbp_player (cast `/Game/TempAssets/Blueprints/Player/BP_Player` OtherActor))
    (`SceneComponent.SetVisibility` (`/Game/TempAssets/Blueprints/Player/BP_Player.Emote Interact` _asbp_player) false false)))

(event `self.ReceiveBeginPlay`
  ;[1 1 1] Declencheur d'évenements
  (bind _asbp_player (cast `/Game/TempAssets/Blueprints/Player/BP_Player` (`GameplayStatics.GetPlayerCharacter` 0)))
  (add `/Game/TempAssets/Blueprints/Player/BP_Player.InteractPressed` _asbp_player (delegate `TriggerEvent`)))

(event `TriggerEvent`
  ;[1 1 1] Declencheur d'évenements
  ;;[1 1 1] Verifier que le joueur soit bien dans la zone
  (if (`self.isPlayerInside`)
    ;;[1 1 1] Executer les interactions de la classe
    (`self.OnInteract`)))

(fn `IsPlayer`
  (params (Object :type "Object Object Reference"))
  (returns (ReturnValue :type Boolean))
  (return (`KismetMathLibrary.ClassIsChildOf` (`GameplayStatics.GetObjectClass` Object) "/Game/TempAssets/Blueprints/Player/BP_Player.BP_Player_C")))

(fn `OnInteract`)

(fn `UserConstructionScript`)