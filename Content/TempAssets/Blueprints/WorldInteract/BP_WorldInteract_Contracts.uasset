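; BP_WorldInteract_Contracts is a world interactable that opens the contract message when the player interacts with it.
; Its OnInteract function passes the Arrow component's world transform to the player character's LookAtMessage with the mesh hidden, then tells the game mode to show the contract message.
; The event graph holds only disabled default nodes, and construction just calls the parent.
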(fn `OnInteract`
  (message `/Game/TempAssets/Blueprints/BPInterfaces/BPI_Character.LookAt` (`GameplayStatics.GetPlayerCharacter` 0) (`SceneComponent.K2_GetComponentToWorld` (`self.Arrow`)) false)
  (message `/Game/TempAssets/Blueprints/BPInterfaces/BPI_Interface.ToggleContract` (`GameplayStatics.GetGameMode`) true))

(fn `UserConstructionScript`
  (`parent.UserConstructionScript`))