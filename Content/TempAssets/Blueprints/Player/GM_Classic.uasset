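; GM_Classic is a game mode that owns the player UI and handles level transitions with a fade.
; On BeginPlay it creates the WBP_Player widget, adds it to the viewport and plays the loading tween in reverse to reveal the game.
; ChangeLevel plays that tween forward, then opens the level when it completes.
; Other events forward slot updates and toggle the contracts and shop panels against the main HUD.
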(event `self.ReceiveBeginPlay`
  ;[0.2552 0.791 1 1 24] Au démarrage du mode de jeu :
  ;;[1 1 1] Initialisation de l'interface générale
  (bind _returnvalue (`|CreateWidget` "/Game/TempAssets/Blueprints/Widgets/WBP_Player.WBP_Player_C"))
  (bind _output_get (set `self.CurrentWBP` _returnvalue))
  (`UserWidget.AddToViewport` _output_get 0)
  ;;[1 1 1] Afficher le jeu
  (`self.FadeOut`))

(event `/Game/TempAssets/Blueprints/BPInterfaces/BPI_Interface.UpdateSlot`
  (params (Index :type Integer) (Percent :type "Float (double-precision)"))
  ;[0.5516 0.5571 1 1 24] Mise à jour de l'interface, pour un slot
  (bind _currentwbp (`self.CurrentWBP`)
    (:`then`
      (`/Game/TempAssets/Blueprints/Widgets/WBP_Player.UpdateSlot` _currentwbp Index Percent))
    (:`else`)))

(event `ChangeLevel`
  (params (Level :type "World Soft Object Reference"))
  ;[0.6172 0.6172 1 1 24] Permet de changer de niveau tout en activant un fondu au noir
  (bind _currentwbp (`self.CurrentWBP`)
    (:`then`
      (`/Game/TempAssets/Blueprints/Widgets/WBP_Player.Play Loading Tween` _currentwbp (delegate `FadeCompleted`) "Forward"))
    (:`else`)))

(event `FadeCompleted`
  ;[0.6172 0.6172 1 1 24] Permet de changer de niveau tout en activant un fondu au noir
  (`GameplayStatics.OpenLevelBySoftObjectPtr` (stale `ChangeLevel` Level)))

(event `FadeOut`
  ;[0.6172 0.6172 1 1 24] Faire un fondu apparent
  (bind _currentwbp (`self.CurrentWBP`)
    (:`then`
      (`/Game/TempAssets/Blueprints/Widgets/WBP_Player.Play Loading Tween` :`self` _currentwbp :`Mode` "Reverse"))
    (:`else`)))

(event `/Game/TempAssets/Blueprints/BPInterfaces/BPI_Interface.ToggleContract`
  (params (Visible :type Boolean))
  ;[0.6172 0.6172 1] Gestion de l'affichage des contrats (GUI)
  (bind _currentwbp (`self.CurrentWBP`)
    (:`then`
      (bind _wbp_contracts (`/Game/TempAssets/Blueprints/Widgets/WBP_Player.WBP_Contracts` _currentwbp))
      (`Widget.SetVisibility` _wbp_contracts (select `bool` Visible :`false` "Hidden" :`true` "Visible" :!type "ESlateVisibility Enum"))
      (`/Game/TempAssets/Blueprints/Widgets/WBP_Contracts.On open` _wbp_contracts)
      (`Widget.SetVisibility` (`/Game/TempAssets/Blueprints/Widgets/WBP_Player.Main_HUD` _currentwbp) (select `bool` Visible :`false` "Visible" :`true` "Hidden" :!type "ESlateVisibility Enum")))
    (:`else`)))

(event `/Game/TempAssets/Blueprints/BPInterfaces/BPI_Interface.ToggleShop`
  (params (Visible :type Boolean))
  ;[0.6172 0.6172 1] Gestion de l'affichage du shop (GUI)
  (bind _currentwbp (`self.CurrentWBP`)
    (:`then`
      (`Widget.SetVisibility` (`/Game/TempAssets/Blueprints/Widgets/WBP_Player.WBP_Shop` _currentwbp) (select `bool` Visible :`false` "Hidden" :`true` "Visible" :!type "ESlateVisibility Enum"))
      (`Widget.SetVisibility` (`/Game/TempAssets/Blueprints/Widgets/WBP_Player.Main_HUD` _currentwbp) (select `bool` Visible :`false` "Visible" :`true` "Hidden" :!type "ESlateVisibility Enum")))
    (:`else`)))

(fn `UserConstructionScript`)