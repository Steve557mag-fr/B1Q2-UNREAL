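; Player character Blueprint with an angled follow camera, Enhanced Input movement, a cooldown-gated dash, weapon use and a pause menu.
; It spawns the current inventory item in the hand socket and forwards primary and secondary attacks to it.
; Timelines scaled by cooldown durations re-enable actions and report progress to the GameMode's UI slots, as does damage.
; Death changes level to HellWorld; Lookat and ResetView override the camera and lock actions.
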(event `Reset Stats`
  ;[0.2706 0.7686 1] Assigner les valeurs par défaut
  (set `self.CurrentHP` (`self.MaxHP`)))

(event `self.ReceiveBeginPlay`
  (bind _returnvalue (pcsubsystem `EnhancedInputLocalPlayerSubsystem` (`GameplayStatics.GetPlayerController` 0)))
  ;[0.2686 0.5645 1 1 35] Au départ :
  ;;[0.1294 0.1294 0.1294] Assigner les contrôles + touches supplémentaires
  (`EnhancedInputSubsystemInterface.AddMappingContext` _returnvalue "/Game/TempAssets/Blueprints/Inputs/IMC_Hero.IMC_Hero" 0 (struct))
  (`EnhancedInputSubsystemInterface.AddMappingContext` _returnvalue "/Game/TempAssets/Blueprints/Inputs/IMC_GameInput.IMC_GameInput" 0 (struct))
  ;;[0.2706 0.7686 1] Initialiser les stats
  (`self.Reset Stats`)
  ;;[1 1 1] Obtenir l'inventaire (une copie)
  (bind _playerdata (message `/Game/TempAssets/Blueprints/BPInterfaces/BPI_GameData.GetPlayerData` (`GameplayStatics.GetGameInstance`)))
  (bind _values (`BlueprintMapLibrary.Map_Values` (`.inventory_25_ACFE1FD54E87585668819288F94517B0` (break `/Game/TempAssets/Blueprints/Structures/GameData/FPlayerData` _playerdata))))
  (set `self.Items` _values)
  (`self.SpawnItem`)
  ;;[1 1 1] Activer la souris et le dash
  (set `PlayerController.bShowMouseCursor` true (`GameplayStatics.GetPlayerController` 0))
  (set `self.CanUseDash` true))

(event `EnhancedInput|/Game/TempAssets/Blueprints/Inputs/IA_Move`
  (params (ActionValue :type "Vector2D Structure") (ElapsedSeconds :type "Float (double-precision)") (TriggeredSeconds :type "Float (double-precision)") (InputAction :type "InputAction Object Reference" :default "/Game/TempAssets/Blueprints/Inputs/IA_Move.IA_Move"))
  (bind _returnvalue (`KismetMathLibrary.MakeRotator` 0.0 0.0 (.yaw (`self.GetControlRotation`))))
  (bind _returnvalue_2 (`KismetMathLibrary.GetForwardVector` _returnvalue))
  (bind _returnvalue_3 (`KismetMathLibrary.GetRightVector` _returnvalue))
  ;[0.9804 0.1137 0.1137 1 35] Mouvements (Déplacement personnage)
  ;;[0.1301 0.1301 0.1301] Déplacement Linéaire (WASD)
  (:`Triggered`
    (if (not (`self.lockPlayerActions`))
      (`self.AddMovementInput` _returnvalue_3 ActionValue_X)
      (`self.AddMovementInput` _returnvalue_2 ActionValue_Y)
      (`SceneComponent.K2_SetRelativeRotation` (`self.Mesh`) (`KismetMathLibrary.MakeRotator` 0.0 0.0 (+ (`KismetMathLibrary.DegAtan2` ActionValue_X ActionValue_Y) -90.0)) false false)))
  (:`Started`
    (set `self.LastDirection` (+ _returnvalue_3 _returnvalue_2))))

(event `EnhancedInput|/Game/TempAssets/Blueprints/Inputs/IA_Dash`
  (params (ActionValue :type Boolean) (ElapsedSeconds :type "Float (double-precision)") (TriggeredSeconds :type "Float (double-precision)") (InputAction :type "InputAction Object Reference" :default "/Game/TempAssets/Blueprints/Inputs/IA_Dash.IA_Dash"))
  ;[0.9804 0.1137 0.1137 1 35] Mouvements (Déplacement personnage)
  ;;[0.1301 0.1301 0.1301] Gestion du Dash
  (:`Started`
    (if (and (`self.CanUseDash`) (not (`self.lockPlayerActions`)))
      (set `self.CanUseDash` false)
      (message `/Game/TempAssets/Blueprints/BPInterfaces/BPI_Interface.UpdateSlot` (`GameplayStatics.GetGameMode`) 1 0.0)
      (`self.LaunchCharacter` (`KismetMathLibrary.MakeVector` (.x (* (`self.DashForce`) (`SceneComponent.GetRightVector` (`self.Mesh`)))) (.y (* (`self.DashForce`) (`SceneComponent.GetRightVector` (`self.Mesh`)))) 250.0))
      (`|PlayMontage` (`self.Mesh`) "/Game/TempAssets/Animations/Player/AM_Dash_v4.AM_Dash_v4"
        (:`then`
          (`TimelineComponent.SetPlayRate` (`self.TL_Dash`) (/ 1.0 (`self.DashCDown`)))
          (bind (_direction _alpha) (`Timeline|TL_Dash` :!via `PlayFromStart`)
            (:`Update`
              (message `/Game/TempAssets/Blueprints/BPInterfaces/BPI_Interface.UpdateSlot` (`GameplayStatics.GetGameMode`) 1 _alpha))
            (:`Finished`
              (set `self.CanUseDash` true))))))))

(event `EnhancedInput|/Game/TempAssets/Blueprints/Inputs/IA_Interact`
  (params (ActionValue :type Boolean) (ElapsedSeconds :type "Float (double-precision)") (TriggeredSeconds :type "Float (double-precision)") (InputAction :type "InputAction Object Reference" :default "/Game/TempAssets/Blueprints/Inputs/IA_Interact.IA_Interact"))
  ;[0.1294 0.1294 0.1294 1 35] Interactions (WI)
  (:`Started`
    (`self.InteractPressed`)))

(event `self.ReceiveAnyDamage`
  (params (Damage :type "Float (single-precision)") (DamageType :type "DamageType Object Reference") (InstigatedBy :type "Controller Object Reference") (DamageCauser :type "Actor Object Reference"))
  ;[0.5474 0.9375 0.3257 1 24] Appliquer les dégats
  (bind _output_get (set `self.CurrentHP` (- (`self.CurrentHP`) Damage)))
  (`GameplayStatics.PlaySound2D` "/Game/TempAssets/SFX/SFX_Player/Got_Hit/SC_Player_Got_Hit.SC_Player_Got_Hit" 1.0 1.0 0.0 null null)
  ;;[1 1 1] Mettre à jour l'interface
  (message `/Game/TempAssets/Blueprints/BPInterfaces/BPI_Interface.UpdateSlot` (`GameplayStatics.GetGameMode`) 2 (/ _output_get (`self.MaxHP`)))
  (if (<= _output_get 0.0)
    (`GameplayStatics.PlaySound2D` "/Game/TempAssets/SFX/SFX_Player/Death/SC_Player_Death.SC_Player_Death" 1.0 1.0 0.0 null null)
    (bind _asgm_classic (cast `/Game/TempAssets/Blueprints/Player/GM_Classic` (`GameplayStatics.GetGameMode`)))
    (`/Game/TempAssets/Blueprints/Player/GM_Classic.ChangeLevel` _asgm_classic "/Game/TempAssets/Levels/Map_HellWorld.Map_HellWorld")))

(event `SpawnItem`
  ;[1 1 1 1 35] Interaction avec l'inventaire
  ;;[1 1 1] Aficher l'arme dans la main
  (bind _currentitem (`self.CurrentItem`)
    (:`then`
      (`self.K2_DestroyActor` _currentitem))
    (:`else`
      _))
  (bind _returnvalue (`|SpawnActorFromClass` (`.item_2_6974B4264218F333DA4182AB32526893` (break `/Game/TempAssets/Blueprints/Structures/GameData/FInventorySlot` (`|GetArrayItem` (`self.Items`) (`self.CurrentSlot`)))) (`KismetMathLibrary.MakeTransform` (0.0 0.0 0.0)) "Undefined" "MultiplyWithRoot" null 5.0 5.0 null))
  (bind _output_get (set `self.CurrentItem` _returnvalue))
  (`self.K2_AttachToComponent` _output_get (`self.Mesh`) (`self.HandSocket`) "KeepRelative" "KeepRelative" "KeepWorld" true)
  ;;[1 1 1] Initaliser l'arme
  (`/Game/TempAssets/Blueprints/Items/BP_Item_Parent.Initialize` (`self.CurrentItem`) self))

(event `EnhancedInput|/Game/TempAssets/Blueprints/Inputs/IA_Attack`
  (params (ActionValue :type Boolean) (ElapsedSeconds :type "Float (double-precision)") (TriggeredSeconds :type "Float (double-precision)") (InputAction :type "InputAction Object Reference" :default "/Game/TempAssets/Blueprints/Inputs/IA_Attack.IA_Attack"))
  ;[1 1 1 1 35] Interaction avec l'inventaire
  ;;[1 1 1] Interaction avec les armes, primaire
  (:`Started`
    (if (not (`self.lockPlayerActions`))
      (bind _currentitem (`self.CurrentItem`)
        (:`then`
          (if (`/Game/TempAssets/Blueprints/Items/BP_Item_Parent.canUse` _currentitem)
            (`/Game/TempAssets/Blueprints/Items/BP_Item_Parent.OnPrimaryBeginUse` _currentitem self)
            (`self.DoCoolDown` 0 _currentitem)))
        (:`else`))))
  (:`Completed`
    (bind _currentitem_2 (`self.CurrentItem`)
      (:`then`
        (`/Game/TempAssets/Blueprints/Items/BP_Item_Parent.OnPrimaryEndUse` _currentitem_2 self))
      (:`else`))))

(event `/Game/TempAssets/Blueprints/BPInterfaces/BPI_Character.LookAt`
  (params (target :type "Transform Structure") (MeshVisible :type Boolean))
  ;[1 1 1] Regarder depuis et vers un emplacement
  (`SceneComponent.K2_SetWorldTransform` (`self.Camera`) target false false)
  (`SceneComponent.SetVisibility` (`self.Mesh`) MeshVisible true)
  (set `self.lockPlayerActions` (not MeshVisible)))

(event `EnhancedInput|/Game/TempAssets/Blueprints/Inputs/IA_RangeAttack`
  (params (ActionValue :type Boolean) (ElapsedSeconds :type "Float (double-precision)") (TriggeredSeconds :type "Float (double-precision)") (InputAction :type "InputAction Object Reference" :default "/Game/TempAssets/Blueprints/Inputs/IA_RangeAttack.IA_RangeAttack"))
  ;[1 1 1 1 35] Interaction avec l'inventaire
  ;;[1 1 1] Interaction avec les armes, secondaire
  (:`Started`
    (if (not (`self.lockPlayerActions`))
      (bind _currentitem (`self.CurrentItem`)
        (:`then`
          (if (`/Game/TempAssets/Blueprints/Items/BP_Item_Parent.canUse` _currentitem)
            (`/Game/TempAssets/Blueprints/Items/BP_Item_Parent.OnSecondaryBeginUse` _currentitem self)
            (`self.DoCoolDown` 0 _currentitem true)))
        (:`else`))))
  (:`Completed`
    (bind _currentitem_2 (`self.CurrentItem`)
      (:`then`
        (`/Game/TempAssets/Blueprints/Items/BP_Item_Parent.OnSecondaryEndUse` _currentitem_2 self))
      (:`else`))))

(event `/Game/TempAssets/Blueprints/BPInterfaces/BPI_Character.ResetView`
  ;[1 1 1] Rénitialiser la vue
  (`self.SetCameraView`)
  (`SceneComponent.SetVisibility` (`self.Mesh`) true true)
  (set `self.lockPlayerActions` false))

(event `EnhancedInput|/Game/TempAssets/Blueprints/Inputs/IA_Pause`
  (params (ActionValue :type Boolean) (ElapsedSeconds :type "Float (double-precision)") (TriggeredSeconds :type "Float (double-precision)") (InputAction :type "InputAction Object Reference" :default "/Game/TempAssets/Blueprints/Inputs/IA_Pause.IA_Pause"))
  ;[1 1 1] Menu Pause
  (:`Started`
    (bind _returnvalue (`|CreateWidget` "/Game/TempAssets/Blueprints/Widgets/WBP_Pause.WBP_Pause_C"))
    (`UserWidget.AddToViewport` _returnvalue 0)
    (set `PlayerController.bShowMouseCursor` true (`GameplayStatics.GetPlayerController` 0))))

(event `DoCoolDown`
  (params (Index :type Integer) (Item :type "/Game/TempAssets/Blueprints/Items/BP_Item_Parent Object Reference") (isSecondary :type Boolean))
  ;[1 1 1] Faire les cooldown avec une animation
  (set `/Game/TempAssets/Blueprints/Items/BP_Item_Parent.canUse` false Item)
  (`TimelineComponent.SetPlayRate` (`self.TL_CoolDown`) (/ 1.0 (select `bool` isSecondary :`false` (`/Game/TempAssets/Blueprints/Items/BP_Item_Parent.PrimaryCDown` Item) :`true` (`/Game/TempAssets/Blueprints/Items/BP_Item_Parent.SecondaryCDown` Item))))
  (bind (_direction _progress) (`Timeline|TL_CoolDown` :!via `PlayFromStart`)
    (:`Update`
      (message `/Game/TempAssets/Blueprints/BPInterfaces/BPI_Interface.UpdateSlot` (`GameplayStatics.GetGameMode`) Index _progress))
    (:`Finished`
      (set `/Game/TempAssets/Blueprints/Items/BP_Item_Parent.canUse` true Item))))

(fn `Get Destination To Range Attack`
  (returns (Destination :type "Vector Structure"))
  (`KismetSystemLibrary.PrintString` "Clic?")
  (return (`.Location` (`GameplayStatics.BreakHitResult` (`PlayerController.GetHitResultUnderCursorByChannel` (`GameplayStatics.GetPlayerController` 0) "TraceTypeQuery2" true)))))

(fn `SetCameraView`
  (bind _cameradistance (`self.CameraDistance`))
  (bind _returnvalue (* _cameradistance (`self.HeightAspect`)))
  (`SceneComponent.K2_SetRelativeLocation` (`self.Camera`) (`KismetMathLibrary.MakeVector` (- 0.0 _cameradistance) 0.0 _returnvalue) false false)
  (`SceneComponent.K2_SetRelativeRotation` (`self.Camera`) (`KismetMathLibrary.MakeRotator` 0.0 (- 0.0 (`KismetMathLibrary.DegAtan2` _returnvalue _cameradistance))) false false))

(fn `UserConstructionScript`
  (`self.SetCameraView`))