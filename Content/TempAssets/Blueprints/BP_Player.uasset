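; BP_Player is the player pawn Blueprint, providing basic ZQSD movement through Enhanced Input.
; BeginPlay adds the IMC_Hero mapping context to the local player's input subsystem.
; IA_Move feeds its X and Y axes into movement along right and forward vectors built from control rotation yaw only, so camera pitch does not affect direction.
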(event `self.ReceiveBeginPlay`
  (`EnhancedInputSubsystemInterface.AddMappingContext` (pcsubsystem `EnhancedInputLocalPlayerSubsystem` (`GameplayStatics.GetPlayerController` 0)) "/Game/TopDownLogic/Blueprints/Input/IMC_Hero.IMC_Hero" 0 (struct)))

(event `EnhancedInput|/Game/TopDownLogic/Blueprints/Input/IA_Move`
  (params (ActionValue :type "Vector2D Structure") (ElapsedSeconds :type "Float (double-precision)") (TriggeredSeconds :type "Float (double-precision)") (InputAction :type "InputAction Object Reference" :default "/Game/TopDownLogic/Blueprints/Input/IA_Move.IA_Move"))
  (bind _returnvalue (`KismetMathLibrary.MakeRotator` 0.0 0.0 (.yaw (`self.GetControlRotation`))))
  ;[0.9804 0.1137 0.1137 1 35] Mouvements (Déplacement personnage)
  ;;[0.1302 0.1302 0.1302] ZQSD Movement input
  (:`Triggered`
    (`self.AddMovementInput` (`KismetMathLibrary.GetRightVector` _returnvalue) ActionValue_X)
    (`self.AddMovementInput` (`KismetMathLibrary.GetForwardVector` _returnvalue) ActionValue_Y)))

(fn `UserConstructionScript`)