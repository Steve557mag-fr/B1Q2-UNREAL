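; A usable item Blueprint that increases the player's walk speed when activated.
; Its Activation override calls the parent, then casts player character 0 to BP_Player and adds SpeedAmount to that character's WalkSpeed.
; The change is a plain additive bump with no timer or revert in this Blueprint, and the event graph holds only disabled default events.
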(fn `Activation`
  (`parent.Activation`)
  (bind _asbp_player (cast `/Game/TempAssets/Blueprints/Player/BP_Player` (`GameplayStatics.GetPlayerCharacter` 0)))
  (set `/Game/TempAssets/Blueprints/Player/BP_Player.WalkSpeed` (+ (`/Game/TempAssets/Blueprints/Player/BP_Player.WalkSpeed` _asbp_player) (`self.SpeedAmount`)) _asbp_player))

(fn `UserConstructionScript`
  (`parent.UserConstructionScript`))