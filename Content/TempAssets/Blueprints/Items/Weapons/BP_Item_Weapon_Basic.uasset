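; Basic weapon item, apparently a scythe, giving the player a melee and a ranged attack.
; Primary use flips the item, plays a montage with notify-toggled Niagara trail, and immediately damages sphere-trace hits along the mesh's right vector.
; Secondary use sphere-traces along the mouse ray, plays another montage, and loops over hits to spawn slash VFX, then after a Delay inside the loop plays sound and applies damage.
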(event `ApplyDamage`
  (bind _mesh (`Character.Mesh` (`self.Player`)))
  (bind _returnvalue (`SceneComponent.K2_GetComponentLocation` _mesh))
  ;[1 0.08333 0.08333 1 24] Attaque
  ;;[1 1 1] Trouver les enemy dans une zone, autour du joueur
  (bind (_outhits _returnvalue_2) (`KismetSystemLibrary.SphereTraceMultiForObjects` _returnvalue (+ _returnvalue (* (`SceneComponent.GetRightVector` _mesh) (`self.Attack_Range`))) (`/Game/TempAssets/Blueprints/Player/BP_Player.AttackRange` (`self.Player`)) (`|MakeArray` "ObjectTypeQuery9" :!type "EObjectTypeQuery Enum") false (`|MakeArray` (`GameplayStatics.GetPlayerCharacter` 0) :!type "Actor Object Reference")))
  ;;[1 1 1] Appliquer les dégats, sur les différents enemies
  (if _returnvalue_2
    (for _array_element _outhits
      (`GameplayStatics.ApplyDamage` (`.HitActor` (`GameplayStatics.BreakHitResult` _array_element)) (`self.Damage`)))))

(event `/Game/TempAssets/Blueprints/Items/BP_Item_Parent.Initialize`
  (params (Player :type "/Game/TempAssets/Blueprints/Player/BP_Player Object Reference"))
  ;[1 1 1 1 24] Quand elle est créé
  (set `self.Player` Player)
  (bind _returnvalue (`NiagaraFunctionLibrary.SpawnSystemAttached` "/Game/TempAssets/VFX/Melee_attack/FXS_Slash_0.FXS_Slash_0" (`self.StaticMesh`) "Scythe_Trail_VFX" (0.0 0.0 0.0) (struct) "KeepRelativeOffset"))
  (bind _output_get (set `self.NS_Attack` _returnvalue))
  (`ActorComponent.Deactivate` _output_get))

(event `/Game/TempAssets/Blueprints/Items/BP_Item_Parent.OnPrimaryBeginUse`
  (params (Player :type "/Game/TempAssets/Blueprints/Player/BP_Player Object Reference"))
  (bind _player (`self.Player`))
  (bind _ns_attack (`self.NS_Attack`))
  ;[1 1 1 1 24] Quand on fait clique-gauche :
  (`self.K2_SetActorRelativeRotation` (`/Game/TempAssets/Blueprints/Player/BP_Player.CurrentItem` Player) (struct :`Yaw` 180.0) false false)
  (bind _notifyname (`|PlayMontage` (`Character.Mesh` _player) "/Game/TempAssets/Animations/Player/AM_Attack0_v4.AM_Attack0_v4" 1.2)
    (:`then`
      (`self.ApplyDamage`))
    (:`OnCompleted`
      (`self.K2_SetActorRelativeRotation` :`self` (`/Game/TempAssets/Blueprints/Player/BP_Player.CurrentItem` _player)))
    (:`OnNotifyBegin`
      (switch `name` _notifyname
        (:`NS_Start`
          (`ActorComponent.Activate` _ns_attack false))
        (:`NS_Stop`
          (`ActorComponent.Deactivate` _ns_attack))))))

(event `/Game/TempAssets/Blueprints/Items/BP_Item_Parent.OnSecondaryBeginUse`
  (params (Player :type "/Game/TempAssets/Blueprints/Player/BP_Player Object Reference"))
  (bind (_worldlocation _worlddirection) (`PlayerController.DeprojectMousePositionToWorld` (`GameplayStatics.GetPlayerController` 0)))
  ;[1 1 1 1 24] Quand on fait clique-droit :
  ;;[1 1 1] On déploie un Sphere cast pour détecter une collision dans un certain rayon
  (bind (_outhits _returnvalue) (`KismetSystemLibrary.SphereTraceMultiForObjects` _worldlocation (+ _worldlocation (* _worlddirection 6000.0)) (`/Game/TempAssets/Blueprints/Player/BP_Player.AttackRange` (`self.Player`)) (`|MakeArray` "ObjectTypeQuery9" :!type "EObjectTypeQuery Enum")))
  ;;[1 1 1] On joue l'animation de l'attque
  (`|PlayMontage` (`Character.Mesh` Player) "/Game/TempAssets/Models/Final/Reaper/V3/AM_Attack1_v3.AM_Attack1_v3"
    (:`then`
      ;;[1 1 1] Si le Sphere cast touche un objet tag "enemy", renvoie un true
      (for _array_element _outhits
        (if _returnvalue
          (bind (_bblockinghit _binitialoverlap _time _distance _location _impactpoint _normal _impactnormal _physmat _hitactor) (`GameplayStatics.BreakHitResult` _array_element))
          ;;[1 1 1] Joue le son et l'animation du SFX
          (bind _returnvalue_2 (`NiagaraFunctionLibrary.SpawnSystemAtLocation` "/Game/TempAssets/VFX/Ranged_attack/FXS_Slash.FXS_Slash" _location (struct) (2.0 2.0 2.0) false))
          (`KismetSystemLibrary.Delay` 0.2)
          (`GameplayStatics.PlaySound2D` "/Game/TempAssets/SFX/SFX_Player/Attacks/Ranged/SC_RangedAttack.SC_RangedAttack" 1.0 1.0 0.0 null null)
          (`ActorComponent.K2_DestroyComponent` _returnvalue_2)
          ;;[1 1 1] Applique les dégats
          (`GameplayStatics.ApplyDamage` _hitactor (`self.Damage`)))))))

(fn `UserConstructionScript`)