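; Base mob Blueprint that chases the player, attacks within range, and reports its death to GI_NomProjet when HP runs out.
; Once StartChase is called, a looping timer repeatedly moves it toward the player until it is in range, then stops it.
; Two timelines, with play rates scaled by configurable delays, time wind-up and recovery around a range-checked damage hit, after which the chase resumes.
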(event `self.ReceiveTick`
  (params (DeltaSeconds :type "Float (single-precision)"))
  (if (`self.Player In Range`)
    _))

(event `StartChase`
  (set `self.CanChase` true)
  (bind _returnvalue (`KismetSystemLibrary.K2_SetTimer` null "OnChase" 0.25 (`self.CanChase`)))
  (set `self.ChaseTimer` _returnvalue))

(event `BeginAttack`
  (`KismetSystemLibrary.PrintString` "Chastre")
  (`TimelineComponent.SetPlayRate` (`self.Timeline Wait Before`) (/ 1.0 (`self.TimeBeforeAttack`)))
  (`Timeline|Timeline Wait Before` :!via `PlayFromStart`
    (:`Finished`
      (`self.Attack`))))

(event `Attack`
  (`self.OnAttack`)
  (`TimelineComponent.SetPlayRate` (`self.Timeline Wait After`) (/ 1.0 (`self.TimeAfterAttack`)))
  (`Timeline|Timeline Wait After` :!via `PlayFromStart`
    (:`Finished`
      (`self.StartChase`))))

(event `self.ReceiveAnyDamage`
  (params (Damage :type "Float (single-precision)") (DamageType :type "DamageType Object Reference") (InstigatedBy :type "Controller Object Reference") (DamageCauser :type "Actor Object Reference"))
  (bind _output_get (set `self.CurrentHP` (- (`self.CurrentHP`) Damage)))
  (`KismetSystemLibrary.PrintString` (`KismetStringLibrary.Conv_DoubleToString` _output_get))
  (if (<= _output_get 0.0)
    (bind _asgi_nom_projet (cast `/Game/TempAssets/Blueprints/GI_NomProjet` (`GameplayStatics.GetGameInstance`)))
    (`/Game/TempAssets/Blueprints/GI_NomProjet.AMobDied` _asgi_nom_projet self)))

(fn `OnAttack`
  (if (`self.Player In Range`)
    (`GameplayStatics.ApplyDamage` (`GameplayStatics.GetPlayerCharacter` 0) (`self.Damage`))))

(fn `OnChase`
  (bind _returnvalue (`GameplayStatics.GetPlayerCharacter` 0))
  (`/Engine/EditorBlueprintResources/StandardMacros.IsValid` _returnvalue
    (:`Is Valid`
      (`AIController.MoveToLocation` (`AIBlueprintHelperLibrary.GetAIController` self) (`self.K2_GetActorLocation` _returnvalue) 0.5 true true false true null true)
      (if (`self.Player In Range`)
        (`MovementComponent.StopMovementImmediately` (`self.CharacterMovement`))
        (`KismetSystemLibrary.K2_ClearAndInvalidateTimerHandle` (`self.ChaseTimer`))
        (set `self.CanChase` false)
        (`self.BeginAttack`)))))

(fn `UserConstructionScript`)