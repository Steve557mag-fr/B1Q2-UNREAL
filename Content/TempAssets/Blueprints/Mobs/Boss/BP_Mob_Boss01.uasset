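; Boss mob for the "Hammarùna" contract that chases on spawn, wields a hand-attached hammer and directly damages the player on attack.
; Runes in the arena scale down incoming damage, blocking it fully at three.
; Crossing two health thresholds decrements the phase and respawns runes at preset locations with enemy spawning disabled.
; At zero health it reports its death, destroys remaining runes and signals contract completion.
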(event `self.ReceiveBeginPlay`
  (`self.StartChase`)
  (message `/Game/TempAssets/Blueprints/BPInterfaces/BPI_WorldEvents.CallNoctification` (`GameplayStatics.GetGameInstance`) "/Game/TempAssets/Blueprints/Widgets/Noctifications/WBP_Noctfication_Attack1.WBP_Noctfication_Attack1_C" 6)
  (`SceneComponent.K2_AttachToComponent` (`self.Hammer`) (`self.Mesh`) "HandR" "KeepRelative" "KeepRelative" "KeepRelative" true))

(event `self.ReceiveAnyDamage`
  (params (Damage :type "Float (single-precision)") (DamageType :type "DamageType Object Reference") (InstigatedBy :type "Controller Object Reference") (DamageCauser :type "Actor Object Reference"))
  ;[1 1 1 1 40] Système de résistance grâce aux rûnes présentes dans la scène
  ;;[0.08235 0.08235 0.08235 1 12] Trouve et récupère le nombre de runes présentes dans l'arène
  (bind _outactors (`GameplayStatics.GetAllActorsOfClass` (`self.RuneClass`)))
  ;;[0.08235 0.08235 0.08235 1 12] Soustrait les dégâts infligés par rapport au nombre de runes restantes, puis les applique aux PVs
  (bind _output_get (set `self.CurrentHP` (- (`self.CurrentHP`) (* Damage (/ (- 3 (`KismetArrayLibrary.Array_Length` _outactors)) 3)))))
  ;;[0.08235 0.08235 0.08235 1 12] Si les PVs sont inférieurs ou égaux à 66, et la phase actuelle est la 3, alors [True >]
  ;;
  ;; Sinon [False >]
  (`KismetSystemLibrary.PrintString` (`KismetStringLibrary.Concat_StrStr` "current HP : " (`KismetStringLibrary.Conv_DoubleToString` _output_get)))
  (if (and (<= _output_get 66.0) (== (`self.Phase`) 3.0))
    ;;[0.08235 0.08235 0.08235 1 12] Passe à la phase suivante
    (`/Engine/EditorBlueprintResources/StandardMacros.DecrementInt` (`self.Phase`)
      (:`  `
        (`self.SpawnRunes` false)))
    (else
      ;;[0.08235 0.08235 0.08235 1 12] Si PVs >= 33 ET Phase == 2 alors [True>]
      ;;
      ;; Sinon [False >]
      (if (and (<= (`self.CurrentHP`) 33.0) (== (`self.Phase`) 2.0))
        ;;[0.08235 0.08235 0.08235 1 12] Passe à la phase suivante
        (`/Engine/EditorBlueprintResources/StandardMacros.DecrementInt` (`self.Phase`)
          (:`  `
            (`self.SpawnRunes` false)))
        (else
          ;;[0.08235 0.08235 0.08235 1 12] Si PVs <= 0 alors le boss est tué + on détruit tt les runes
          (if (<= (`self.CurrentHP`) 0.0)
            (message `/Game/TempAssets/Blueprints/BPInterfaces/BPI_WorldEvents.OnEnemyDied` (`GameplayStatics.GetGameInstance`) self)
            (bind _outactors_2 (`GameplayStatics.GetAllActorsOfClass` "/Game/TempAssets/Models/Final/Rune/A_Rune.A_Rune_C"))
            (for _array_element _outactors_2
              (`self.K2_DestroyActor` _array_element))
            (message `/Game/TempAssets/Blueprints/BPInterfaces/BPI_Interface.ContractFinished` (`GameplayStatics.GetGameMode`) "Hammarùna")))))))

(event `SpawnRunes`
  (params (SpawnEnemies :type Boolean))
  ;[1 1 1 1 40] Système de résistance grâce aux rûnes présentes dans la scène
  ;;[0.08235 0.01759 0.01759 1 15] Spawn des runes
  ;;;[0.08235 0.08235 0.08235 1 12] Définit la position (dans Locations) du spawn des runes
  (for _array_element (`self.Locations`)
    ;;;[0.08235 0.08235 0.08235 1 12] Spawn les runes et leur attribue le spawn des ennemis (BP_Rune dans RuneClass)
    (bind _returnvalue (`|SpawnActorFromClass` (`self.RuneClass`) (`KismetMathLibrary.MakeTransform` _array_element) "Undefined" "MultiplyWithRoot" null null))
    (set `/Game/TempAssets/Models/Final/Rune/A_Rune.CanSpawnEnemies` SpawnEnemies _returnvalue)))

(event `PlayAMAttack`
  (`|PlayMontage` (`self.Mesh`) "/Game/TempAssets/Animations/Boss1/AM_Attack.AM_Attack"))

(fn `OnAttack`
  (`self.PlayAMAttack`)
  (if true
    (`GameplayStatics.ApplyDamage` (`GameplayStatics.GetPlayerCharacter` 0) (`self.Damage`))))

(fn `UserConstructionScript`
  (`parent.UserConstructionScript`))