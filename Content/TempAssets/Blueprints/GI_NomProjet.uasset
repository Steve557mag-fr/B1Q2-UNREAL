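; Game Instance that owns the player's persistent save: souls, contracts and inventory, plus game settings.
; It loads or creates a BP_GameSlot on Init, writes it to disk on Shutdown, and exposes getters for player data and settings.
; Events edit the save in memory, validating new contracts and items against DataTables and stacking item amounts in a map.
; A MobDied event destroys the dead enemy's actor.
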(event `self.ReceiveShutdown`
  ;[1 1 1] DEBUG SAVING
  (`self.SaveToDisk` (`self.defaultSlot`))
  (`KismetSystemLibrary.PrintString` "Saved!"))

(event `self.ReceiveInit`
  ;[1 1 1] Lire les données sur le disque au démarrage
  (`self.LoadFromDisk` (`self.defaultSlot`)))

(event `/Game/TempAssets/Blueprints/BPInterfaces/BPI_GameData.AddSouls`
  (params (amount :type Integer))
  (bind _playerdata (`/Game/TempAssets/Blueprints/BP_GameSlot.PlayerData` (`self.SaveSlot`)))
  ;[1 1 1] Permet de donner une quantité d’âme au joueur
  ;;[1 1 1] Ajouter au total d'âme, la quantité
  (setmembers `/Game/TempAssets/Blueprints/Structures/GameData/FPlayerData` :`StructRef` _playerdata :`souls` (+ amount (`.souls_10_F5A24C85444C62EAEF13B7818743067E` (break `/Game/TempAssets/Blueprints/Structures/GameData/FPlayerData` _playerdata)))))

(event `/Game/TempAssets/Blueprints/BPInterfaces/BPI_GameData.AddContract`
  (params (contractName :type String))
  (bind _playerdata (`/Game/TempAssets/Blueprints/BP_GameSlot.PlayerData` (`self.SaveSlot`)))
  (bind ((`contracts_19_43B3594E451C55A4239B7F9AE65FC263` _contracts)) (break `/Game/TempAssets/Blueprints/Structures/GameData/FPlayerData` _playerdata))
  ;[1 1 1] Permet d’ajouter un contrat au joueur, grâce son ID.
  ;;[1 1 1] Si le contrat existe dans le DataTable et que le contrat n'est pas déjà pris, on le rajoute à la liste des contrats
  (bind _returnvalue (`DataTableFunctionLibrary.DoesDataTableRowExist` "/Game/TempAssets/Data/DT_Contracts.DT_Contracts" (`KismetStringLibrary.Conv_StringToName` contractName)))
  (if _returnvalue
    (`BlueprintSetLibrary.Set_Add` _contracts contractName)
    (setmembers `/Game/TempAssets/Blueprints/Structures/GameData/FPlayerData` :`StructRef` _playerdata :`contracts` _contracts)))

(event `/Game/TempAssets/Blueprints/BPInterfaces/BPI_GameData.AddItem`
  (params (itemName :type String))
  (bind _returnvalue (`KismetStringLibrary.Conv_StringToName` itemName))
  (bind _playerdata (`/Game/TempAssets/Blueprints/BP_GameSlot.PlayerData` (`self.SaveSlot`)))
  (bind ((`inventory_25_ACFE1FD54E87585668819288F94517B0` _inventory)) (break `/Game/TempAssets/Blueprints/Structures/GameData/FPlayerData` _playerdata))
  (bind _value (`BlueprintMapLibrary.Map_Find` _inventory _returnvalue))
  ;[1 1 1] Ajouter un item à l'inventaire du joueur
  ;;[1 1 1] Si l'item existe dans la table des items
  (bind _returnvalue_2 (`DataTableFunctionLibrary.DoesDataTableRowExist` "/Game/TempAssets/Data/DT_Items.DT_Items" _returnvalue))
  (if _returnvalue_2
    ;;[1 1 1] Obtenir l'item à rajouter dans l'inventaire
    (bind _returnvalue_3 (`|GetDataTableRow` "/Game/TempAssets/Data/DT_Items.DT_Items" _returnvalue)
      (:`then`
        ;;[1 1 1] Verifier si l'item existe déjà
        (if (`BlueprintMapLibrary.Map_Contains` _inventory _returnvalue)
          (bind ((`item_8_B4FB166043B98F1E214092B2A7E1E1CA` _item)) (break `/Game/TempAssets/Blueprints/Structures/FItemRow` _returnvalue_3))
          ;;[1 1 1] Si oui, ajouter la quantité
          (bind _structout (setmembers `/Game/TempAssets/Blueprints/Structures/GameData/FInventorySlot` :`StructRef` _value :`amount` (+ (`.amount_8_FE147153450A42373832649E3755602C` (break `/Game/TempAssets/Blueprints/Structures/GameData/FInventorySlot` _value)) (`.amount_8_FE147153450A42373832649E3755602C` (break `/Game/TempAssets/Blueprints/Structures/GameData/FInventorySlot` _item)))))
          (`BlueprintMapLibrary.Map_Add` _inventory _returnvalue _structout)
          (else
            ;;[1 1 1] Sinon, ajouter l'item à la map
            (`BlueprintMapLibrary.Map_Add` _inventory _returnvalue _item)))
        (setmembers `/Game/TempAssets/Blueprints/Structures/GameData/FPlayerData` :`StructRef` _playerdata :`inventory` _inventory)))))

(event `/Game/TempAssets/Blueprints/BPInterfaces/BPI_GameData.FinishContract`
  (params (contractName :type String))
  (bind _playerdata (`/Game/TempAssets/Blueprints/BP_GameSlot.PlayerData` (`self.SaveSlot`)))
  (bind ((`contracts_19_43B3594E451C55A4239B7F9AE65FC263` _contracts)) (break `/Game/TempAssets/Blueprints/Structures/GameData/FPlayerData` _playerdata))
  ;[1 1 1] Permet de finir (donc retirer) un contrat selon son nom.
  ;;[1 1 1] Verifier si le contrat était présent
  (if (`BlueprintSetLibrary.Set_Contains` _contracts contractName)
    ;;[1 1 1] Si oui, on le supprime + joue l'animation de contrat achevé
    (`BlueprintSetLibrary.Set_Remove` _contracts contractName)
    (setmembers `/Game/TempAssets/Blueprints/Structures/GameData/FPlayerData` :`StructRef` _playerdata :`contracts` _contracts)))

(event `/Game/TempAssets/Blueprints/BPInterfaces/BPI_GameData.UpdateItem`
  (params (itemName :type Name) (amount :type Integer))
  (bind _playerdata (`/Game/TempAssets/Blueprints/BP_GameSlot.PlayerData` (`self.SaveSlot`)))
  (bind ((`inventory_25_ACFE1FD54E87585668819288F94517B0` _inventory)) (break `/Game/TempAssets/Blueprints/Structures/GameData/FPlayerData` _playerdata))
  (bind (_value _returnvalue) (`BlueprintMapLibrary.Map_Find` _inventory itemName))
  (bind ((`infinte_5_E763FBFD42E557E8E5095A8557493960` _infinte) (`amount_8_FE147153450A42373832649E3755602C` _amount)) (break `/Game/TempAssets/Blueprints/Structures/GameData/FInventorySlot` _value))
  (bind _returnvalue_2 (- _amount (* (`KismetMathLibrary.Conv_BoolToInt` _infinte) amount)))
  ;[1 1 1] Permet de mettre à jour l’état d’un item, grâce à son nom (dans la table TD_Items).
  ;;[1 1 1] Vérifier et trouver si l'item existe
  (if _returnvalue
    ;;[1 1 1] Si la quantité est > 0, on diminue juste la quantité
    (if (> _returnvalue_2 0)
      (bind _structout (setmembers `/Game/TempAssets/Blueprints/Structures/GameData/FInventorySlot` :`StructRef` _value :`amount` _returnvalue_2))
      (`BlueprintMapLibrary.Map_Add` _inventory itemName _structout)
      (else
        ;;[1 1 1] Sinon, on retire l'item
        (`BlueprintMapLibrary.Map_Remove` _inventory itemName)))
    (setmembers `/Game/TempAssets/Blueprints/Structures/GameData/FPlayerData` :`StructRef` _playerdata :`inventory` _inventory)))

(event `[DISPATCH] MobDied`
  (params (Mob :type "/Game/TempAssets/Blueprints/Mobs/BP_Mob_Pareent Object Reference"))
  ;[1 1 1] Quand un ennemi meurt :
  (`Actor.K2_DestroyActor` Mob))

(fn `GetGameSettings`
  (returns (GameSettings :type "/Game/TempAssets/Blueprints/Structures/GameData/FGameSettings Structure"))
  (if (`self.isLoaded`)
    (return (`/Game/TempAssets/Blueprints/BP_GameSlot.GameSettings` (`self.SaveSlot`)))
    (else
      (return))))

(fn `GetPlayerData`
  (returns (PlayerData :type "/Game/TempAssets/Blueprints/Structures/GameData/FPlayerData Structure"))
  (return (`/Game/TempAssets/Blueprints/BP_GameSlot.PlayerData` (`self.SaveSlot`))))

(fn `LoadFromDisk`
  (params (slotName :type String))
  ;[1 1 1] Vérifier si la sauvegarde existe
  (bind _returnvalue (`GameplayStatics.DoesSaveGameExist` slotName))
  (if _returnvalue
    ;[1 1 1] Charger si elle existe (+ cast en GameSlot pour sauver dans le BP dans 'SaveSlot')
    (bind _returnvalue_2 (`GameplayStatics.LoadGameFromSlot` slotName))
    (bind _asbp_game_slot (cast `/Game/TempAssets/Blueprints/BP_GameSlot` _returnvalue_2))
    (set `self.SaveSlot` _asbp_game_slot)
    (else
      ;[1 1 1] Sinon, Créer un nouveau GameSlot (+ le sauver dans le BP dans 'SaveSlot')
      (bind _returnvalue_3 (`GameplayStatics.CreateSaveGameObject` "/Game/TempAssets/Blueprints/BP_GameSlot.BP_GameSlot_C"))
      (set `self.SaveSlot` _returnvalue_3)))
  (set `self.isLoaded` true)
  (return))

(fn `SaveToDisk`
  (params (SlotName :type String))
  ;[1 1 1] Verifier si on a une sauvegarde chargée
  (if (not (`self.isLoaded`))
    ;[1 1 1] Charger la sauvegarde si elle n'est pas chargée
    (`self.LoadFromDisk` SlotName))
  ;[1 1 1] Sauver le 'GameSlot' sur le disque
  (`GameplayStatics.SaveGameToSlot` (`self.SaveSlot`) SlotName)
  (return))