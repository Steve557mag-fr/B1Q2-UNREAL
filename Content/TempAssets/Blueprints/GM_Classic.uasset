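; Game mode that creates the player HUD and handles faded transitions between levels.
; BeginPlay adds WBP_Player to the viewport, then plays its loading tween in reverse to reveal the game.
; ChangeLevel plays that tween forward with a completion delegate that opens the requested level by object reference.
; UpdateAll forwards to UpdateHealth, which is a stub that only checks the widget's validity.
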(event `self.ReceiveBeginPlay`
  ;[0.2552 0.791 1] Au démarrage du mode de jeu :
  ;;[1 1 1] Initialisation de l'interface générale
  (bind _returnvalue (`|CreateWidget` "/Game/TempAssets/Blueprints/Widgets/WBP_Player.WBP_Player_C"))
  (bind _output_get (set `self.CurrentWBP` _returnvalue))
  (`UserWidget.AddToViewport` _output_get 0)
  ;;[1 1 1] Afficher le jeu
  (`self.FadeOut`))

(event `self.UpdateAll`
  (`self.UpdateHealth`))

(event `self.UpdateHealth`
  (`self.CurrentWBP`
    (:`then`)
    (:`else`)))

(event `ChangeLevel`
  (params (Level :type "World Soft Object Reference"))
  (bind _currentwbp (`self.CurrentWBP`)
    (:`then`
      (`/Game/TempAssets/Blueprints/Widgets/WBP_Player.Play Loading Tween` _currentwbp (delegate `FadeCompleted`) "Forward"))
    (:`else`)))

(event `FadeCompleted`
  (`GameplayStatics.OpenLevelBySoftObjectPtr` (stale `ChangeLevel` Level)))

(event `FadeOut`
  (bind _currentwbp (`self.CurrentWBP`)
    (:`then`
      (`/Game/TempAssets/Blueprints/Widgets/WBP_Player.Play Loading Tween` :`self` _currentwbp :`Mode` "Reverse"))
    (:`else`)))

(fn `UserConstructionScript`)