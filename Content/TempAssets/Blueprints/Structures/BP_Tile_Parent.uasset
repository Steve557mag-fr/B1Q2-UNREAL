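; BP_Tile_Parent is a base structure tile that spawns its terrain and describes its connection points to other pieces.
; CreateTile spawns RefBPP at a world position, saves it as CurrentInstance and attaches it to the tile.
; Connections come from GetMap, a placeholder here, and are looked up by arrow name or by normalized local direction within a tolerance.
; Arrow components represent connections: GetArrows reads the instance's arrows, and DestroyConnection removes arrows by name.
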(event `CreateTile`
  (params (WPosition :type "Vector Structure"))
  ;[1 1 1] Permet de créer la tuile (physiquement dans le monde)
  (bind _returnvalue (`|SpawnActorFromClass` (`self.RefBPP`) (`KismetMathLibrary.MakeTransform` WPosition) "Undefined" "MultiplyWithRoot" null null))
  ;;[1 1 1] Sauver l'instance
  (bind _output_get (set `self.CurrentInstance` _returnvalue))
  (`self.K2_AttachToActor` _output_get self "None" "KeepWorld" "KeepWorld" "KeepWorld" true))

(event `DestroyConnection`
  (params (Connection :type String))
  ;[1 1 1] Permet de détruire une connexion parmis les connections de l'instance
  (for _array_element (`self.K2_GetComponentsByClass` "/Script/Engine.ArrowComponent")
    (if (`KismetStringLibrary.EqualEqual_StrStr` (`KismetSystemLibrary.GetObjectName` _array_element) Connection)
      (`ActorComponent.K2_DestroyComponent` _array_element))))

(fn `Get Map`
  (returns (Map :type "Array of /Game/TempAssets/Blueprints/DataStructs/FConnection Structure"))
  (return (`|MakeArray` (struct) :!type "/Game/TempAssets/Blueprints/DataStructs/FConnection Structure")))

(fn `GetArrows`
  (returns (Out :type "Array of ArrowComponent Object Reference") (isEmpty :type Boolean))
  (bind _currentinstance (`self.CurrentInstance`))
  (bind _returnvalue (`self.K2_GetComponentsByClass` _currentinstance "/Script/Engine.ArrowComponent"))
  ;[1 1 1] Si le terrain de la tuile n'existe pas, on retourne rien + IsEmpty à vrai.
  (`/Engine/EditorBlueprintResources/StandardMacros.IsValid` _currentinstance
    (:`Is Valid`
      ;[1 1 1] Sinon, récupérer les flèches sur le terrain + isEmpty selon si la liste est vide ou pas
      (return _returnvalue (`KismetArrayLibrary.Array_IsEmpty` _returnvalue)))
    (:`Is Not Valid`
      (return _ true))))

(fn `GetConnectionByDirection`
  (params (Direction :type "Vector Structure"))
  (returns (Connection :type "/Game/TempAssets/Blueprints/DataStructs/FConnection Structure") (Find :type Boolean))
  ;[1 1 1] Pour chaque connexion
  (for _array_element (`self.Get Map`)
    ;;[1 1 1] Verifier si la direction est la ==
    (if (== (`KismetMathLibrary.Normal` Direction) (`KismetMathLibrary.Normal` (.location (`.ArrowLocal_13_E013388D4BB038E1DEA2BC81170D86DB` (break `/Game/TempAssets/Blueprints/DataStructs/FConnection` _array_element)))) :`ErrorTolerance` 0.1)
      (return _array_element true)))
  (return (struct) false))

(fn `GetConnectionByName`
  (params (Name :type String))
  (returns (Connection :type "/Game/TempAssets/Blueprints/DataStructs/FConnection Structure") (Find :type Boolean))
  (for _array_element (`self.Get Map`)
    (bind _returnvalue (`KismetStringLibrary.EqualEqual_StrStr` (`.ArrowName_20_379168A1401FFDD92D1801A2DAC50E5E` (break `/Game/TempAssets/Blueprints/DataStructs/FConnection` _array_element)) Name))
    (if _returnvalue
      (return _array_element _returnvalue)))
  (return (struct) false))

(fn `UserConstructionScript`)