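; BP_Tile_Plain is a plain structure tile that describes its connection points for tile-based layouts.
; GetMap adds an entry to CurrentMap for each of its four valid Arrow components, then returns the map.
; Each entry holds the arrow's name, world and relative transforms, and an array containing only BP_Tile_Plain.
; BeginPlay and the construction script only call the parent.
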(event `self.ReceiveBeginPlay`
  (`parent.ReceiveBeginPlay`))

(fn `Get Map`
  (returns (Map :type "Array of /Game/TempAssets/Blueprints/DataStructs/FIncludeTiles Structure"))
  (locals (CurrentMap :type "Array of /Game/TempAssets/Blueprints/DataStructs/FIncludeTiles Structure"))
  (bind _arrow_0 (`self.Arrow_0`))
  (bind _arrow_1 (`self.Arrow_1`))
  (bind _arrow_2 (`self.Arrow_2`))
  (bind _arrow_3 (`self.Arrow_3`))
  ;[1 1 1] Permet de récuperer les informations lié aux connexions
  (`|ExecutionSequence`
    (:`then_0`
      (`/Engine/EditorBlueprintResources/StandardMacros.IsValid` _arrow_0
        (:`Is Valid`
          (`KismetArrayLibrary.Array_Add` (`local.CurrentMap`) (make `/Game/TempAssets/Blueprints/DataStructs/FIncludeTiles` (`KismetSystemLibrary.GetObjectName` _arrow_0) (`SceneComponent.K2_GetComponentToWorld` _arrow_0) (`SceneComponent.GetRelativeTransform` _arrow_0) (`|MakeArray` "BP_Tile_Plain_C" :!type "/Game/TempAssets/Blueprints/Structures/BP_Tile_Parent Class Reference"))))))
    (:`then_1`
      (`/Engine/EditorBlueprintResources/StandardMacros.IsValid` _arrow_1
        (:`Is Valid`
          (`KismetArrayLibrary.Array_Add` (`local.CurrentMap`) (make `/Game/TempAssets/Blueprints/DataStructs/FIncludeTiles` (`KismetSystemLibrary.GetObjectName` _arrow_1) (`SceneComponent.K2_GetComponentToWorld` _arrow_1) (`SceneComponent.GetRelativeTransform` _arrow_1) (`|MakeArray` "BP_Tile_Plain_C" :!type "/Game/TempAssets/Blueprints/Structures/BP_Tile_Parent Class Reference"))))))
    (:`then_2`
      (`/Engine/EditorBlueprintResources/StandardMacros.IsValid` _arrow_2
        (:`Is Valid`
          (`KismetArrayLibrary.Array_Add` (`local.CurrentMap`) (make `/Game/TempAssets/Blueprints/DataStructs/FIncludeTiles` (`KismetSystemLibrary.GetObjectName` _arrow_2) (`SceneComponent.K2_GetComponentToWorld` _arrow_2) (`SceneComponent.GetRelativeTransform` _arrow_2) (`|MakeArray` "BP_Tile_Plain_C" :!type "/Game/TempAssets/Blueprints/Structures/BP_Tile_Parent Class Reference"))))))
    (:`then_3`
      (`/Engine/EditorBlueprintResources/StandardMacros.IsValid` _arrow_3
        (:`Is Valid`
          (`KismetArrayLibrary.Array_Add` (`local.CurrentMap`) (make `/Game/TempAssets/Blueprints/DataStructs/FIncludeTiles` (`KismetSystemLibrary.GetObjectName` _arrow_3) (`SceneComponent.K2_GetComponentToWorld` _arrow_3) (`SceneComponent.GetRelativeTransform` _arrow_3) (`|MakeArray` "BP_Tile_Plain_C" :!type "/Game/TempAssets/Blueprints/Structures/BP_Tile_Parent Class Reference"))))))
    (:`then_4`
      (return (`local.CurrentMap`)))))

(fn `UserConstructionScript`
  (`parent.UserConstructionScript`))