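; GM_WorldGame, apparently a game mode, procedurally builds the world from tile-based structures on BeginPlay.
; CreateWorld chooses the default structure or, by a Chance roll, a random one from a shrinking pool, then passes it to SpawnStructure with an origin.
; SpawnStructure spawns a random number of copies of the structure's first tile at that origin.
; Generation looks unfinished: connection matching does nothing, origins are cleared without refilling, and RandomGetTile is never called.
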(event `self.ReceiveBeginPlay`
  (`self.CreateWorld` null 1 (`self.WorldStructures`)))

(event `CreateWorld`
  (params (OriginPostion :type "ArrowComponent Object Reference") (MaxStructures :type Integer :default 1) (Structures :type "Array of /Game/TempAssets/Blueprints/Structures/Structure_Default/BP_Structure_Default Class Reference"))
  (bind _currentstructure (`self.CurrentStructure`))
  (bind _finaloriginpositions (`self.FinalOriginPositions`))
  ;[1 1 1] APIREF:NOTION
  ;;[1 1 1] Initialiser les variables
  (set `self.FinalOriginPositions` (`|MakeArray` OriginPostion))
  (set `self.CurrentStructures` Structures)
  ;;[1 1 1] Faire X structures ...
  (for _ (range (+ MaxStructures 1))
    ;;[1 1 1] Prendre une structure aléatoirement
    (set `self.CurrentStructure` (`self.DefaultStructure`))
    (if (not (>= (`KismetMathLibrary.RandomInteger` 100) (`self.chance`)))
      (bind _structure (`self.PickFromCurrentStructures`))
      (set `self.CurrentStructure` _structure))
    ;;[1 1 1] Faire apparaitre la structure choisie
    (if (`KismetSystemLibrary.IsValidClass` _currentstructure)
      (`self.SpawnStructure` _currentstructure (`|GetArrayItem` _finaloriginpositions (`KismetMathLibrary.RandomInteger` (`KismetArrayLibrary.Array_Length` _finaloriginpositions)))))))

(fn `PickFromCurrentStructures`
  (returns (Structure :type "/Game/TempAssets/Blueprints/Structures/Structure_Default/BP_Structure_Default Class Reference"))
  (bind _currentstructures (`self.CurrentStructures`))
  (bind _returnvalue (`KismetArrayLibrary.Array_Length` _currentstructures))
  (bind _returnvalue_2 (`KismetMathLibrary.RandomInteger` _returnvalue))
  (bind _output (`|GetArrayItem` _currentstructures _returnvalue_2))
  (if (== _returnvalue 0)
    (return null)
    (else
      (`KismetArrayLibrary.Array_Remove` _currentstructures _returnvalue_2)
      ;[1 1 1] debug
      (`KismetSystemLibrary.PrintString` (`KismetSystemLibrary.GetClassDisplayName` _output))
      (return _output))))

(fn `RandomGetTile`
  (params (ExcludeTile :type "Array of /Game/TempAssets/Blueprints/Structures/BP_Tile_Parent Class Reference") (Structure :type "/Game/TempAssets/Blueprints/Structures/BP_Structure_Parent Class Reference"))
  (returns (OutTile :type "/Game/TempAssets/Blueprints/Structures/BP_Tile_Parent Class Reference"))
  (locals (iteration :type Integer) (currentTile :type "/Game/TempAssets/Blueprints/Structures/BP_Tile_Parent Class Reference"))
  (bind _tiles (defaults `Object` Structure))
  (bind _currenttile (`local.currentTile`))
  (bind _returnvalue (< (`local.iteration`) 10))
  (set `local.iteration` 0)
  (while (and _returnvalue (or (`KismetArrayLibrary.Array_Contains` ExcludeTile _currenttile) (`KismetSystemLibrary.IsValidClass` _currenttile)))
    (set `local.currentTile` (`|GetArrayItem` _tiles (`KismetMathLibrary.RandomInteger` (`KismetArrayLibrary.Array_Length` _tiles))))
    (`/Engine/EditorBlueprintResources/StandardMacros.IncrementInt` (`local.iteration`)))
  (if _returnvalue
    (return (`local.currentTile`))
    (else
      (return null))))

(fn `SpawnStructure`
  (params (Structure :type "/Game/TempAssets/Blueprints/Structures/Structure_Default/BP_Structure_Default Class Reference") (LastOrigin :type "ArrowComponent Object Reference"))
  (returns (BossSpawned :type Boolean))
  (bind (_maxtiles _tiles) (defaults `Object` Structure))
  (bind _currentarrows (`self.CurrentArrows`))
  (set `self.CurrentArrows` (`|MakeArray` LastOrigin))
  (for _ (range (+ (`KismetMathLibrary.RandomIntegerInRange` 1 _maxtiles) 1))
    (bind _returnvalue (`|SpawnActorFromClass` (`|GetArrayItem` _tiles) (`KismetMathLibrary.MakeTransform` (`SceneComponent.K2_GetComponentLocation` (`|GetArrayItem` _currentarrows (`KismetMathLibrary.RandomInteger` (`KismetArrayLibrary.Array_Length` _currentarrows))))) "Undefined" "MultiplyWithRoot" null null))
    (`KismetArrayLibrary.Array_Clear` (`self.FinalOriginPositions`))
    (for _array_element (`/Game/TempAssets/Blueprints/Structures/BP_Tile_Parent.Connections` _returnvalue)
      (if (== (* (`SceneComponent.GetForwardVector` _array_element) -1) (0.0 0.0 0.0))
        _)))
  (return false))

(fn `UserConstructionScript`)